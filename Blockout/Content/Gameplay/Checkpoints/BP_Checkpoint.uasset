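; BP_Checkpoint is a placeable checkpoint that hands its respawn data to the game mode when the player reaches it.
; On BeginPlay it packs its label, the world transform of its RespawnTransform component and its collectables to respawn into a CheckpointData struct.
; An overlap of its Collision by a Player-tagged actor passes that struct to the game mode through SaveNewCheckpointMessage.
; The construction script writes the label to CheckpointLabel as text.
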(event OnComponentBeginOverlap(Collision)
  (params (OverlappedComponent :type Primitive%20Component%20Object%20Reference) (OtherActor :type Actor%20Object%20Reference) (OtherComp :type Primitive%20Component%20Object%20Reference) (OtherBodyIndex :type Integer) (bFromSweep :type Boolean) (SweepResult :type Hit%20Result%20Structure%20%28by%20ref%29))
  ;[1 1 1] Begin overlap
  (if (Actor|ActorHasTag OtherActor "Player")
    (Class|BPIGameMode|SaveNewCheckpoint(Message) (Game|GetGameMode) (Variables|Data|GetCheckpointData))))

(event EventBeginPlay
  ;[0.3894 1 0.3256] Begin play
  (bind _structout (Utilities|Struct|SetmembersinStruct_CheckpointData (Variables|Data|GetCheckpointData) (Variables|Settings|GetLabel) (Transformation|GetWorldTransform (Variables|Default|GetRespawnTransform)) (Variables|Settings|GetCollectablesToRespawn)))
  (Variables|Data|SetCheckpointData _structout))

(fn ConstructionScript
  (Rendering|Components|TextRender|SetText (Variables|Default|GetCheckpointLabel) (Utilities|Text|ToText(String) (Variables|Settings|GetLabel))))