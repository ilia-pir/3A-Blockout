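; Timed platform that drops and fades out after a tagged player stands on it for a set time, showing a countdown through the game mode.
; Stepping off early cancels the timer and re-arms it.
; One timeline lerps location and dynamic-material alpha, disables collision after the fall, and plays in reverse to respawn.
; Respawn runs on a timer or, with RespawnThroughTrigger, through TriggerReceiver, with DoOnce gates blocking repeats.
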(event OnComponentBeginOverlap(Collision)
  (params (OverlappedComponent :type Primitive%20Component%20Object%20Reference) (OtherActor :type Actor%20Object%20Reference) (OtherComp :type Primitive%20Component%20Object%20Reference) (OtherBodyIndex :type Integer) (bFromSweep :type Boolean) (SweepResult :type Hit%20Result%20Structure%20%28by%20ref%29))
  ;[1 1 1] Begin overlap
  (if (Actor|ActorHasTag OtherActor "Player")
    ;[1 1 1] Fall timer
    (Utilities|FlowControl|DoOnce false
      (:Completed
        (bind _returnvalue (Utilities|Time|SetTimerbyEvent (delegate Custom|PlattformFall) (Variables|Settings|GetTimeTillFall)))
        (Variables|Timer|SetFallTimer _returnvalue)
        (Class|BPIGameMode|ShowHideGlobalCountdown(Message) (Game|GetGameMode) (Variables|Settings|GetTimeTillFall) true)))))

(event OnComponentEndOverlap(Collision)
  (params (OverlappedComponent :type Primitive%20Component%20Object%20Reference) (OtherActor :type Actor%20Object%20Reference) (OtherComp :type Primitive%20Component%20Object%20Reference) (OtherBodyIndex :type Integer))
  ;[1 1 1] End overlap
  (if (Actor|ActorHasTag OtherActor "Player")
    (if (Utilities|Time|IsTimerActivebyHandle (Variables|Timer|GetFallTimer))
      (Utilities|Time|ClearandInvalidateTimerbyHandle (Variables|Timer|GetFallTimer))
      (Class|BPIGameMode|ShowHideGlobalCountdown(Message) (Game|GetGameMode) 0.0 false)
      (CallFunction|PlattformReset))))

(event Custom|PlattformFall
  ;[1 1 1] Fall timer
  (CallFunction|TogglePlattform true)
  (if (not (Variables|Settings|GetbRespawnThroughTrigger))
    ;[1 1 1] Respawn
    (Utilities|Time|SetTimerbyEvent (delegate Custom|RespawnPlattform) (Variables|Settings|GetRespawnTime))))

(event Custom|TogglePlattform
  (params (bHide :type Boolean))
  (bind _basecolor (Variables|Data|GetBaseColor))
  ;[1 1 1] Toggle Plattform
  (if bHide
    (bind (_direction _alpha_0_1) (Timeline|PlattformFade PlayFromStart)
      (:Update
        ;[1 1 1] Plattform Movement
        (Transformation|SetWorldLocation (Variables|Default|GetPlattform) (Math|Vector|Lerp(Vector) (Variables|Data|GetPlattformStartLocation) (- (Variables|Data|GetPlattformStartLocation) (* (Math|Vector|GetUpVector (Variables|Default|GetPlattform)) (Variables|Settings|GetFallDistance))) _alpha_0_1) false false)
        ;[1 1 1] Color Fade
        (Rendering|Material|SetVectorParameterValue (Variables|Materials|GetDMI_Plattform) "Color" (Utilities|Struct|MakeLinearColor (.r _basecolor) (.g _basecolor) (.b _basecolor) (- 1.0 _alpha_0_1)) :!class /Script/Engine.MaterialInstanceDynamic))
      (:Finished
        ;[1 1 1] Plattform timeline finish
        (switch Utilities|FlowControl|Switch|SwitchonETimelineDirection _direction
          (:Forward
            (Collision|SetCollisionEnabled (Variables|Default|GetPlattform) "NoCollision")
            (if (Variables|Settings|GetbRespawnThroughTrigger)
              (CallFunction|ResetTriggerFadein)))
          (:Backward
            (Collision|SetCollisionEnabled (Variables|Default|GetPlattform) "QueryAndPhysics")
            (CallFunction|PlattformReset)))))
    (else
      (Timeline|PlattformFade ReverseFromEnd))))

(event Custom|RespawnPlattform
  ;[1 1 1] Respawn
  (CallFunction|TogglePlattform false))

(event Custom|PlattformReset
  ;[1 1 1] Fall timer
  (Utilities|FlowControl|DoOnce false) ; enters at Reset
)

(event Custom|ResetTriggerFadeIn
  ;[1 1 1] Trigger fade in
  (Utilities|FlowControl|DoOnce true) ; enters at Reset
)

(event EventBeginPlay
  ;[0.4681 1 0.3554] Begin play
  (bind _returnvalue (Rendering|Material|GetVectorParameterValue (Variables|Materials|GetDMI_Plattform) "Color" :!class /Script/Engine.MaterialInstanceDynamic))
  (Variables|Data|SetBaseColor _returnvalue)
  (Variables|Data|SetPlattformStartLocation (Transformation|GetWorldLocation (Variables|Default|GetPlattform)))
  (Components|Timeline|SetPlayRate (Variables|Default|GetPlattformFade) (Variables|Settings|GetPlattformFadeRate)))

(event EventTriggerReceiver
  (params (bTriggersOnce :type Boolean))
  ;[1 1 1] Trigger fade in
  (if (Variables|Settings|GetbRespawnThroughTrigger)
    (Utilities|FlowControl|DoOnce true
      (:Completed
        (CallFunction|TogglePlattform false)))))

(fn ConstructionScript
  (bind _returnvalue (Rendering|Material|CreateDynamicMaterialInstance (Variables|Default|GetPlattform) 0 (Rendering|Material|GetMaterial (Variables|Default|GetPlattform) 0) "None" :!class /Script/Engine.PrimitiveComponent))
  (Variables|Materials|SetDMI_Plattform _returnvalue))